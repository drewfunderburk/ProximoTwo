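; BP_Button_ToggleLights is an interactable button that toggles the visibility of chosen lights on other actors.
; On BeginPlay it resolves each component reference in ActorsWithLightsToToggle by matching component names on the referenced actor, then caches the light components in ComponentsToToggle.
; OnInteract flips the visibility of each cached light without propagating to child components.
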(event EventBeginPlay
  ;[1 1 1] Cache Lights
  (for _array_element (Variables|Default|GetActors%20with%20Lights%20to%20Toggle)
    (for _array_element_2 (Actor|GetComponentsByClass (.otheractor _array_element) "/Script/Engine.ActorComponent")
      (if (== (Utilities|GetObjectName _array_element_2) (.componentproperty _array_element))
        (bind _aslight_component (Utilities|Casting|CastToLightComponent _array_element_2))
        (Utilities|Array|AddUnique (Variables|Default|GetComponents%20To%20Toggle) _aslight_component)))))

(event EventOnInteract
  ;[1 1 1] Toggle Lights
  (for _array_element (Variables|Default|GetComponents%20To%20Toggle)
    (Rendering|ToggleVisibility _array_element false)))

(fn ConstructionScript)