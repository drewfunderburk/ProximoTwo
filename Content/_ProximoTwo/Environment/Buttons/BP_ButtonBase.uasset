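; BP_ButtonBase is a button actor that relays interactions to a list of other objects in the level.
; On interact, it passes the source on to each entry in InteractableObjects that implements the Interactable interface.
; When DrawLineToObjects is enabled, Tick draws green debug lines from the button to each listed object to show the links.
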(event EventTick
  (params (DeltaSeconds :type Float%20%28single-precision%29))
  (if (Variables|Default|GetDrawLineToObjects)
    (for _array_element (Variables|Default|GetInteractable%20Objects)
      (Rendering|Debug|DrawDebugLine (Transformation|GetActorLocation) (Transformation|GetActorLocation _array_element) "(R=0.000000,G=1.000000,B=0.000000,A=1.000000)" 0.0 0.0))))

(event EventOnInteract
  (params (source :type Actor%20Object%20Reference))
  (for _array_element (Variables|Default|GetInteractable%20Objects)
    (if (Utilities|DoesObjectImplementInterface _array_element "/Script/ProximoTwo.Interactable")
      (Class|Interactable|OnInteract(Message) _array_element source))))

(fn ConstructionScript)