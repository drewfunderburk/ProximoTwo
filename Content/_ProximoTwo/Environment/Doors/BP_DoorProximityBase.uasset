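; BP_DoorProximityBase is a base proximity trigger for doors, built around a box volume.
; Begin and end overlaps on the box broadcast OnDoorOpen and OnDoorClose with the overlapping actor, with no filtering, leaving the door's response to whatever listens.
; When the DrawDebug flag is set, Tick draws the box's scaled, rotated bounds in green.
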(event OnComponentBeginOverlap(Box)
  (params (OverlappedComponent :type Primitive%20Component%20Object%20Reference) (OtherActor :type Actor%20Object%20Reference) (OtherComp :type Primitive%20Component%20Object%20Reference) (OtherBodyIndex :type Integer) (bFromSweep :type Boolean) (SweepResult :type Hit%20Result%20Structure%20%28by%20ref%29))
  (Default|CallOnDoorOpen OtherActor))

(event OnComponentEndOverlap(Box)
  (params (OverlappedComponent :type Primitive%20Component%20Object%20Reference) (OtherActor :type Actor%20Object%20Reference) (OtherComp :type Primitive%20Component%20Object%20Reference) (OtherBodyIndex :type Integer))
  (Default|CallOnDoorClose OtherActor))

(event EventTick
  (params (DeltaSeconds :type Float%20%28single-precision%29))
  (CallFunction|DrawDebug (Variables|Default|GetDraw%20Debug)))

(fn ConstructionScript)

(fn DrawDebug
  (params (Draw? :type Boolean))
  (if Draw?
    (Rendering|Debug|DrawDebugBox)))