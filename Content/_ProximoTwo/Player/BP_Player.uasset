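; Player character Blueprint that adds a crosshair widget on BeginPlay, forwards Primary Fire to CallOnFire and handles smooth crouching.
; Crouch press, gated by CanCrouch, lowers walk speed and plays a timeline that lerps capsule half-height.
; Release only flags WantsToUncrouch; the separate OnUncrouch event, not triggered in these graphs, restores speed and reverses the timeline.
; Tick optionally draws the capsule for debugging.
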(event EventTick
  (params (DeltaSeconds :type Float%20%28single-precision%29))
  (Rendering|Debug|DrawDebugCapsule (Variables|Default|GetDraw%20Debug%20Capsule)))

(event EventBeginPlay
  (|AddCrosshairWidget))

(event Input|ActionEvents|InputActionPrimaryFire
  (params (Key :type Key%20Structure :default "None"))
  (:Pressed
    (Default|CallOnFire)))

(fn ConstructionScript)

(event EventOnUncrouch
  (Variables|/Script/Engine.CharacterMovementComponent|SetMaxWalkSpeed (Variables|Character|GetCharacterMovement) (Variables|Default|GetbaseWalkSpeed))
  (Variables|Default|SetisCrouched false)
  (bind _lerp (Timeline|CrouchTimeline Reverse)
    (:Update
      (|LerpCrouch _lerp))))

(event Input|ActionEvents|InputActionCrouch
  (params (Key :type Key%20Structure :default "None"))
  (bind _charactermovement (Variables|Character|GetCharacterMovement))
  (:Pressed
    (if (Class|Character|CanCrouch)
      (Variables|Default|SetisCrouched true)
      (Variables|/Script/Engine.CharacterMovementComponent|SetMaxWalkSpeed _charactermovement (Variables|/Script/Engine.CharacterMovementComponent|GetMaxWalkSpeedCrouched _charactermovement))
      (bind _lerp (Timeline|CrouchTimeline Play)
        (:Update
          (|LerpCrouch _lerp)))))
  (:Released
    (Variables|Default|SetwantsToUncrouch true)))